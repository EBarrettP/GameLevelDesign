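; Blood blob NPC that emerges a spike limb and repeatedly stabs at the player, triggering DamageEffect when its hit volume overlaps them.
; AttackSequence loops tracking, target snapshot, wind-up, strike and reset, or strikes around a fixed position in fake-attack mode.
; Timeline lerps drive limb motion and whole-blob relocation, with yaw derived from the target's clamped X offset.
; A ribbon beam endpoint and wavy dynamic material shape its look.
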(event OnComponentBeginOverlap(HitCheck)
  (params (OverlappedComponent :type Primitive%20Component%20Object%20Reference) (OtherActor :type Actor%20Object%20Reference) (OtherComp :type Primitive%20Component%20Object%20Reference) (OtherBodyIndex :type Integer) (bFromSweep :type Boolean) (SweepResult :type Hit%20Result%20Structure%20%28by%20ref%29))
  (if (== OtherActor (Variables|Default|GetPlayer))
    (Default|DamageEffect (Variables|Default|GetPlayer))))

(event Custom|AttackSequence
  ;[0.05208 0.05208 0.05208] Attack Functions
  ;;[0.7771 1 0.8046] Attack Sequence
  (if (Variables|Default|GetAttacking)
    (CallFunction|FollowPlayerTarget)
    (Utilities|FlowControl|Delay 4.0)
    (CallFunction|TargettoPlayer)
    (CallFunction|RotatetoTarget :!label _label)
    (Utilities|FlowControl|Delay 0.9)
    (else
      (CallFunction|TargettoPosition)
      (if (Variables|TargetRotation|GetTurnToTarget)
        (goto _label)
        (else
          _))))
  (CallFunction|Attack)
  (Utilities|FlowControl|Delay 1.0)
  (CallFunction|ResetAttack)
  (Utilities|FlowControl|Delay 1.0)
  (if (or (Variables|Default|GetAttacking) (Variables|Default|GetFakeAttacking))
    (CallFunction|AttackSequence)))

(event Custom|RotateToTarget
  ;[0.05208 0.05208 0.05208] Attack Functions
  ;;[1 0.5608 0.08235] Rotate to target
  (CallFunction|GetDifference true)
  (Audio|PlaySoundatLocation "/Engine/VREditor/Sounds/VR_ungrab.VR_ungrab" (Variables|LocationTracking|GetSpikeDefaultLocation) "0, 0, 0" 0.5 0.001 0.15 0 0 0 0)
  (if (Variables|Default|GetFakeAttacking)
    (Variables|TargetRotation|SetTargetRotateX 1.6e+02)
    (bind _newtrack_0 (Timeline|RotateTimeline PlayFromStart)
      (:Update
        (Transformation|SetRelativeRotation (Variables|Default|GetAttackLimb) (Math|Rotator|MakeRotator (.x (Math|Vector|Lerp(Vector) (Variables|TargetRotation|GetCurrentRotation) (Math|Vector|MakeVector (Variables|TargetRotation|GetTargetRotateX) 0.0 (Variables|TargetRotation|GetTurn)) _newtrack_0)) 0.0 (.z (Math|Vector|Lerp(Vector) (Variables|TargetRotation|GetCurrentRotation) (Math|Vector|MakeVector (Variables|TargetRotation|GetTargetRotateX) 0.0 (Variables|TargetRotation|GetTurn)) _newtrack_0))) false false)))
    (else
      (Variables|TargetRotation|SetTargetRotateX 1.2e+02)
      (Timeline|RotateTimeline PlayFromStart))))

(event Custom|Attack
  (bind _attacklimb (Variables|Default|GetAttackLimb))
  ;[0.05208 0.05208 0.05208] Attack Functions
  ;;[0.5677 0.07392 0.07392] Attack
  (bind _newtrack_0 (Timeline|AttackTimeline PlayFromStart)
    (:Update
      (Transformation|SetWorldLocation _attacklimb (Math|Vector|Lerp(Vector) (Transformation|GetWorldLocation _attacklimb) (Transformation|GetActorLocation (Variables|TargetRotation|GetTargetPoint)) _newtrack_0) false false))
    (:Finished
      (CallFunction|SetCurrentRotation))))

(event Custom|ResetAttack
  (bind _attacklimb (Variables|Default|GetAttackLimb))
  ;[0.05208 0.05208 0.05208] Attack Functions
  ;;[0.153 0.3703 0.625] Reset
  (bind _newtrack_0 (Timeline|ResetTimeline PlayFromStart)
    (:Update
      (Transformation|SetWorldLocation _attacklimb (Math|Vector|Lerp(Vector) (Transformation|GetWorldLocation _attacklimb) (Variables|LocationTracking|GetSpikeDefaultLocation) _newtrack_0) false false)
      (Transformation|SetRelativeRotation (Variables|Default|GetAttackLimb) (Math|Rotator|MakeRotator (.x (Math|Vector|Lerp(Vector) (Variables|TargetRotation|GetCurrentRotation) (Math|Vector|MakeVector 1.1e+02 0.0 0.0) _newtrack_0)) 0.0 (.z (Math|Vector|Lerp(Vector) (Variables|TargetRotation|GetCurrentRotation) (Math|Vector|MakeVector 1.1e+02 0.0 0.0) _newtrack_0))) false false))
    (:Finished
      (CallFunction|SetCurrentRotation))))

(event Custom|TargetToPosition
  (bind _returnvalue (Math|Random|RandomFloatinRange -5e+01 5e+01))
  (bind _fakeattackposition (Variables|LocationTracking|GetFakeAttackPosition))
  ;[0.05208 0.05208 0.05208] Attack Functions
  ;;[0.34 0.23 0.19] Move target to position
  (Transformation|SetActorLocation (Variables|TargetRotation|GetTargetPoint) (Math|Vector|MakeVector (+ (.x _fakeattackposition) _returnvalue) (+ (.y _fakeattackposition) _returnvalue) (.z _fakeattackposition)) false false))

(event Custom|ReadyToAttack
  ;[0.1206 0.1289 0.1302] Prepare to Attack
  (Variables|LocationTracking|SetSpikeStartLocation (Transformation|GetWorldLocation (Variables|Default|GetAttackLimb)))
  (bind _newtrack_2 (Timeline|EmergeTimeline PlayFromStart)
    (:Update
      (Transformation|SetWorldLocation (Variables|Default|GetAttackLimb) (Math|Vector|Lerp(Vector) (Variables|LocationTracking|GetSpikeStartLocation) (+ (Variables|LocationTracking|GetSpikeStartLocation) (Variables|LocationTracking|GetSpikeMoveTo)) _newtrack_2) false false))
    (:Finished
      (Variables|LocationTracking|SetSpikeDefaultLocation (Transformation|GetWorldLocation (Variables|Default|GetAttackLimb)))
      (CallFunction|SetCurrentRotation)
      (Variables|Default|SetAttacking true)
      (CallFunction|AttackSequence))))

(event Custom|GetDifference
  (params (TargetPoint :type Boolean))
  ;[0.05208 0.05208 0.05208] Attack Functions
  ;;[1 0.5608 0.08235] Target Rotation Calculation
  (if TargetPoint
    (Variables|TargetRotation|SetTargetX (.x (Transformation|GetActorLocation (Variables|TargetRotation|GetTargetPoint))))
    (else
      (Variables|TargetRotation|SetTargetX (.x (Transformation|GetActorLocation (Variables|Default|GetPlayer))))))
  (Variables|TargetRotation|SetDefaultX (.x (Transformation|GetWorldLocation (Variables|Default|GetRotationBox))))
  (if (>= (Variables|TargetRotation|GetTargetX) (Variables|TargetRotation|GetDefaultX))
    (Variables|TargetRotation|SetDifference (- (Variables|TargetRotation|GetTargetX) (Variables|TargetRotation|GetDefaultX)))
    (Variables|TargetRotation|SetTurn -1.0)
    (Variables|TargetRotation|SetTurnMultiplier 5.0) ; PlayerRight
    (Variables|TargetRotation|SetTurn (Math|Float|Clamp(Float) (- (* (Variables|TargetRotation|GetTurn) (/ (Variables|TargetRotation|GetDifference) (Variables|TargetRotation|GetTurnMultiplier))) -3e+01) -5e+01 3e+01))
    (else
      (Variables|TargetRotation|SetDifference (- (Variables|TargetRotation|GetDefaultX) (Variables|TargetRotation|GetTargetX)))
      (Variables|TargetRotation|SetTurn 1.0)
      (Variables|TargetRotation|SetTurnMultiplier 3.5)
      (Variables|TargetRotation|SetTurn (Math|Float|Clamp(Float) (- (* (Variables|TargetRotation|GetTurn) (/ (Variables|TargetRotation|GetDifference) (Variables|TargetRotation|GetTurnMultiplier))) -3e+01) 0.0 1e+02)))))

(event Custom|MoveEntire
  ;[0.1406 0.1406 0.1406] Move Entire Blob
  (bind _output_get (Variables|LocationTracking|SetMoveStartLocation (Transformation|GetActorLocation)))
  (bind _newtrack_0 (Timeline|CompleteMoveTimeL PlayFromStart)
    (:Update
      (Transformation|SetActorLocation (Math|Vector|Lerp(Vector) _output_get (Variables|LocationTracking|GetMoveToLocation) _newtrack_0) false false))
    (:Finished
      (Variables|LocationTracking|SetSpikeDefaultLocation (Transformation|GetWorldLocation (Variables|Default|GetAttackLimb)))
      (Effects|Components|ParticleSystem|SetVectorParameter (Variables|Default|GetRibbon) "Beam End" (Transformation|GetWorldLocation (Variables|Default|GetRibbonEnd)))
      (CallFunction|AttackSequence))))

(event Custom|SetCurrentRotation
  (bind _attacklimb (Variables|Default|GetAttackLimb))
  (bind _relativerotation (Variables|/Script/Engine.SceneComponent|GetRelativeRotation _attacklimb))
  ;[0.05208 0.05208 0.05208] Attack Functions
  (Variables|TargetRotation|SetCurrentRotation (Math|Vector|MakeVector (.roll _relativerotation) 0.0 (.yaw _relativerotation))))

(event Custom|FollowPlayerTarget
  ;[0.05208 0.05208 0.05208] Attack Functions
  ;;[0.1667 0.02083 0.09256] Spike follows the player
  (bind _newtrack_0 (Timeline|TargetTimeline PlayFromStart)
    (:Update
      (CallFunction|GetDifference false)
      (if (>= _newtrack_0 1.0)
        (Transformation|SetRelativeRotation (Variables|Default|GetAttackLimb) (Math|Rotator|MakeRotator 1.1e+02 0.0 (Variables|TargetRotation|GetTurn)) false false)
        (else
          (Transformation|SetRelativeRotation (Variables|Default|GetAttackLimb) (Math|Rotator|MakeRotator (.x (Math|Vector|Lerp(Vector) (Variables|TargetRotation|GetCurrentRotation) (Math|Vector|MakeVector 1.1e+02 0.0 (Variables|TargetRotation|GetTurn)) _newtrack_0)) 0.0 (.z (Math|Vector|Lerp(Vector) (Variables|TargetRotation|GetCurrentRotation) (Math|Vector|MakeVector 1.1e+02 0.0 (Variables|TargetRotation|GetTurn)) _newtrack_0))) false false))))
    (:Finished
      (CallFunction|SetCurrentRotation))))

(event Custom|TargetToPlayer
  (bind _targetpoint (Variables|TargetRotation|GetTargetPoint))
  (bind _player (Variables|Default|GetPlayer))
  (bind _returnvalue (Transformation|GetActorLocation _player))
  ;[0.05208 0.05208 0.05208] Attack Functions
  ;;[0.34 0.23 0.19] Move target to player
  (Transformation|SetActorLocation _targetpoint (Math|Vector|MakeVector (.x _returnvalue) (.y _returnvalue) (.z (Transformation|GetActorLocation _targetpoint))) false false))

(event EventBeginPlay
  (Effects|Components|ParticleSystem|SetVectorParameter (Variables|Default|GetRibbon) "Beam End" (Transformation|GetWorldLocation (Variables|Default|GetRibbonEnd)))
  (bind _returnvalue (Actor|GetActorOfClass "/Game/ThirdPerson/Blueprints/BP_ThirdPersonCharacter.BP_ThirdPersonCharacter_C"))
  (Variables|Default|SetPlayer _returnvalue))

(fn ConstructionScript
  (bind _returnvalue (Rendering|Material|CreateDynamicMaterialInstance "/Game/LevelAssets/Materials/WavyBloodMat.WavyBloodMat" "None" "None" :!class /Script/Engine.KismetMaterialLibrary))
  (bind _output_get (Variables|Default|SetWaveInst _returnvalue))
  (Rendering|Material|SetMaterial (Variables|Default|GetCentralSphere) 0 _output_get)
  (Rendering|Material|SetScalarParameterValueonMaterials (Variables|Default|GetCentralSphere) "WaveHeight" 1e+01))