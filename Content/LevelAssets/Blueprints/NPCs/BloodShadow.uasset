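; BloodShadow is a decal-based NPC that acts as one step in an ordered flood sequence run by FloodManager.
; Approaching it early triggers a Lunge that reveals a skeletal mesh and, after a delay, damages the player if still in range.
; Overlap also gates interact input: at its turn, interacting activates its water plane, advances the sequence, then fades the decal's dynamic material and destroys the actor.
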(event OnComponentBeginOverlap(Box)
  (params (OverlappedComponent :type Primitive%20Component%20Object%20Reference) (OtherActor :type Actor%20Object%20Reference) (OtherComp :type Primitive%20Component%20Object%20Reference) (OtherBodyIndex :type Integer) (bFromSweep :type Boolean) (SweepResult :type Hit%20Result%20Structure%20%28by%20ref%29))
  (bind _floodmanager (Variables|References|GetFloodManager))
  (if (Actor|ActorHasTag OtherActor "Player")
    (Variables|References|SetPlayer OtherActor)
    (if (>= (Variables|/Game/LevelAssets/Blueprints/Functions/Managers/FloodManager.FloodManager_C|GetSequenceNumber (Variables|References|GetFloodManager)) (Variables|Sequence|GetNumberInSequence))
      (Default|ShowText (Variables|References|GetUIManager))
      (else
        (Variables|Default|SetInAttackRange true)
        (CallFunction|Lunge)))
    (Input|EnableInput (Game|GetPlayerController 0))
    (Utilities|FlowControl|Gate true) ; enters at Open
  ))

(event OnComponentEndOverlap(Box)
  (params (OverlappedComponent :type Primitive%20Component%20Object%20Reference) (OtherActor :type Actor%20Object%20Reference) (OtherComp :type Primitive%20Component%20Object%20Reference) (OtherBodyIndex :type Integer))
  (bind _floodmanager (Variables|References|GetFloodManager))
  (if (Actor|ActorHasTag OtherActor "Player")
    (Variables|Default|SetInAttackRange false)
    (Default|RemoveText (Variables|References|GetUIManager))
    (Input|DisableInput (Game|GetPlayerController 0))
    (Utilities|FlowControl|Gate true) ; enters at Close
  ))

(event Custom|Lunge
  (if (not (Variables|Default|GetAttacking))
    (Variables|Default|SetAttacking true)
    (Rendering|Material|SetScalarParameterValue (Variables|References|GetMatInst) "RenderHalf?" 1.0 :!class /Script/Engine.MaterialInstanceDynamic)
    (Development|SetHiddeninGame (Variables|Default|GetSkeletalMesh) false false)
    (Components|Animation|PlayAnimation (Variables|Default|GetSkeletalMesh) "/Game/LevelAssets/Meshes+Animation/LungeAnim.LungeAnim" false)
    (Audio|PlaySoundatLocation "/Engine/VREditor/Sounds/VR_ungrab.VR_ungrab" (Transformation|GetWorldLocation (Variables|Default|GetSkeletalMesh)) "0, 0, 0" 0.3 0.001 0.15 0 0 0 0)
    (Utilities|FlowControl|Delay 1.07)
    (if (Variables|Default|GetInAttackRange)
      (bind _asbp_third_person_character (Utilities|Casting|CastToBP_ThirdPersonCharacter (Variables|References|GetPlayer)))
      (Default|DamageEffect _asbp_third_person_character))
    (Utilities|FlowControl|Delay 1.2)
    (Rendering|Material|SetScalarParameterValue (Variables|References|GetMatInst) "RenderHalf?" 0.0 :!class /Script/Engine.MaterialInstanceDynamic)
    (Development|SetHiddeninGame (Variables|Default|GetSkeletalMesh) true false)
    (Variables|Default|SetAttacking false)))

(event EventBeginPlay
  (bind _returnvalue (Actor|GetActorOfClass "/Game/LevelAssets/Blueprints/Functions/Managers/UIManager.UIManager_C"))
  (Variables|References|SetUIManager _returnvalue)
  (bind _returnvalue_2 (Actor|GetActorOfClass "/Game/LevelAssets/Blueprints/Functions/Managers/FloodManager.FloodManager_C"))
  (Variables|References|SetFloodManager _returnvalue_2))

(event Input|ActionEvents|InputActionInteract
  (params (Key :type Key%20Structure :default "None"))
  (bind _floodmanager (Variables|References|GetFloodManager))
  (:Pressed
    (Utilities|FlowControl|Gate true
      (:Exit
        (if (== (Variables|/Game/LevelAssets/Blueprints/Functions/Managers/FloodManager.FloodManager_C|GetSequenceNumber (Variables|References|GetFloodManager)) (Variables|Sequence|GetNumberInSequence))
          (Default|MakeWaterActive _floodmanager (Variables|Default|GetWaterPlane))
          (Default|SequenceUp _floodmanager)
          (Audio|PlaySoundatLocation "/Engine/VREditor/Sounds/VR_grab.VR_grab" (Transformation|GetActorLocation) "0, 0, 0" 0.1 0.01 0.0 0 0 0 0)
          (bind _newtrack_0 (Timeline|FadeTimeline PlayFromStart)
            (:Update
              (Rendering|Material|SetScalarParameterValue (Variables|References|GetMatInst) "Opacity" _newtrack_0 :!class /Script/Engine.MaterialInstanceDynamic))
            (:Finished
              (Actor|DestroyActor)))
          (else
            (CallFunction|Lunge)))))))

(fn ConstructionScript
  (bind _returnvalue (Rendering|Material|CreateDynamicMaterialInstance (Variables|Default|GetDecal) :!class /Script/Engine.DecalComponent))
  (bind _output_get (Variables|References|SetMatInst _returnvalue))
  (Rendering|Components|Decal|SetDecalMaterial (Variables|Default|GetDecal) _output_get))