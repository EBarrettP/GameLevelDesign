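; Big blood blob enemy that starts hidden until activated, damages the player on contact, and bursts and is destroyed if touched while the player is rock-merged.
; Its looping attack sequence tracks the player with the limb, locks a target point, winds up, lunges and resets, or strikes a preset position for fake attacks.
; Timelines lerp the limb's motion, with turn derived from the target's clamped X offset.
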(event OnComponentBeginOverlap(HitCheck)
  (params (OverlappedComponent :type Primitive%20Component%20Object%20Reference) (OtherActor :type Actor%20Object%20Reference) (OtherComp :type Primitive%20Component%20Object%20Reference) (OtherBodyIndex :type Integer) (bFromSweep :type Boolean) (SweepResult :type Hit%20Result%20Structure%20%28by%20ref%29))
  (bind _returnvalue (Transformation|GetActorTransform))
  (bind _player (Variables|Default|GetPlayer))
  (if (== OtherActor (Variables|Default|GetPlayer))
    (if (Variables|/Game/ThirdPerson/Blueprints/BP_ThirdPersonCharacter.BP_ThirdPersonCharacter_C|GetRockMerged _player)
      (Niagara|SpawnSystematLocation "/Game/LevelAssets/ParticleEffects/BloodBurst.BloodBurst" (.location _returnvalue) (.rotation _returnvalue) (.scale _returnvalue))
      (Default|RockEnd (Variables|Default|GetPlayer))
      (Actor|DestroyActor)
      (else
        (Default|DamageEffect _player)))))

(event Custom|AttackSequence
  ;[0.05208 0.05208 0.05208] Attack Functions
  ;;[0.7771 1 0.8046] Attack Sequence
  (if (Variables|Default|GetAttacking)
    (CallFunction|FollowPlayerTarget)
    (Utilities|FlowControl|Delay 4.0)
    (CallFunction|TargettoPlayer)
    (CallFunction|RotatetoTarget :!label _label)
    (Utilities|FlowControl|Delay 0.9)
    (else
      (CallFunction|TargettoPosition)
      (if (Variables|Default|GetTurnToTarget)
        (goto _label)
        (else
          _))))
  (CallFunction|Attack)
  (Utilities|FlowControl|Delay 1.0)
  (CallFunction|ResetAttack)
  (Utilities|FlowControl|Delay 1.0)
  (if (or (Variables|Default|GetAttacking) (Variables|Default|GetFakeAttacking))
    (CallFunction|AttackSequence)))

(event Custom|Activate
  (Rendering|SetActorHiddenInGame false)
  (Collision|SetActorEnableCollision true)
  (Effects|Components|ParticleSystem|SetVectorParameter (Variables|Default|GetRibbon) "Beam End" (Transformation|GetWorldLocation (Variables|Default|GetRibbonEnd)))
  (Rendering|Material|SetMaterial (Variables|/Script/Engine.StaticMeshActor|GetStaticMeshComponent (Variables|Default|GetPlane)) 0 "/Game/LevelAssets/Materials/WavelessBloodMat.WavelessBloodMat"))

(event Custom|RotateToTarget
  ;[0.05208 0.05208 0.05208] Attack Functions
  ;;[1 0.5608 0.08235] Rotate to target
  (CallFunction|GetDifference true)
  (Audio|PlaySoundatLocation "/Engine/VREditor/Sounds/VR_ungrab.VR_ungrab" (Variables|LocationTracking|GetSpikeDefaultLocation) "0, 0, 0" 0.3 0.001 0.15 0 0 0 0)
  (if (Variables|Default|GetFakeAttacking)
    (Variables|Default|SetTargetRotateX 9e+01)
    (bind _newtrack_0 (Timeline|RotateTimeline PlayFromStart)
      (:Update
        (Transformation|SetRelativeRotation (Variables|Default|GetAttackLimb) (Math|Rotator|MakeRotator (.x (Math|Vector|Lerp(Vector) (Variables|TargetRotation|GetCurrentRotation) (Math|Vector|MakeVector (Variables|Default|GetTargetRotateX) 0.0 (Variables|TargetRotation|GetTurn)) _newtrack_0)) 0.0 (.z (Math|Vector|Lerp(Vector) (Variables|TargetRotation|GetCurrentRotation) (Math|Vector|MakeVector (Variables|Default|GetTargetRotateX) 0.0 (Variables|TargetRotation|GetTurn)) _newtrack_0))) false false)))
    (else
      (Variables|Default|SetTargetRotateX 1.3e+02)
      (Timeline|RotateTimeline PlayFromStart))))

(event Custom|Attack
  (bind _attacklimb (Variables|Default|GetAttackLimb))
  ;[0.05208 0.05208 0.05208] Attack Functions
  ;;[0.5677 0.07392 0.07392] Attack
  (bind _newtrack_0 (Timeline|AttackTimeline PlayFromStart)
    (:Update
      (Transformation|SetWorldLocation _attacklimb (Math|Vector|Lerp(Vector) (Transformation|GetWorldLocation _attacklimb) (Transformation|GetActorLocation (Variables|TargetRotation|GetTargetPoint)) _newtrack_0) false false))
    (:Finished
      (CallFunction|SetCurrentRotation))))

(event Custom|ResetAttack
  (bind _attacklimb (Variables|Default|GetAttackLimb))
  ;[0.05208 0.05208 0.05208] Attack Functions
  ;;[0.153 0.3703 0.625] Reset
  (bind _newtrack_0 (Timeline|ResetTimeline PlayFromStart)
    (:Update
      (Transformation|SetWorldLocation _attacklimb (Math|Vector|Lerp(Vector) (Transformation|GetWorldLocation _attacklimb) (Variables|LocationTracking|GetSpikeDefaultLocation) _newtrack_0) false false)
      (Transformation|SetRelativeRotation (Variables|Default|GetAttackLimb) (Math|Rotator|MakeRotator (.x (Math|Vector|Lerp(Vector) (Variables|TargetRotation|GetCurrentRotation) (Math|Vector|MakeVector 1e+02 0.0 0.0) _newtrack_0)) 0.0 (.z (Math|Vector|Lerp(Vector) (Variables|TargetRotation|GetCurrentRotation) (Math|Vector|MakeVector 1e+02 0.0 0.0) _newtrack_0))) false false))
    (:Finished
      (CallFunction|SetCurrentRotation))))

(event Custom|TargetToPosition
  (bind _fakeattackposition (Variables|Default|GetFakeAttackPosition))
  ;[0.05208 0.05208 0.05208] Attack Functions
  ;;[0.34 0.23 0.19] Move target to position
  (Transformation|SetActorLocation (Variables|TargetRotation|GetTargetPoint) (Math|Vector|MakeVector (.x _fakeattackposition) (.y _fakeattackposition) (.z _fakeattackposition)) false false))

(event Custom|GetDifference
  (params (TargetPoint :type Boolean))
  ;[0.05208 0.05208 0.05208] Attack Functions
  ;;[1 0.5608 0.08235] Target Rotation Calculation
  (if TargetPoint
    (Variables|TargetRotation|SetTargetX (.x (Transformation|GetActorLocation (Variables|TargetRotation|GetTargetPoint))))
    (else
      (Variables|TargetRotation|SetTargetX (.x (Transformation|GetActorLocation (Variables|Default|GetPlayer))))))
  (Variables|TargetRotation|SetDefaultX (.x (Transformation|GetWorldLocation (Variables|Default|GetRotationBox))))
  (if (>= (Variables|TargetRotation|GetTargetX) (Variables|TargetRotation|GetDefaultX))
    (Variables|TargetRotation|SetDifference (- (Variables|TargetRotation|GetTargetX) (Variables|TargetRotation|GetDefaultX)))
    (Variables|TargetRotation|SetTurn -1.0)
    (Variables|Default|SetTurnMultiplier 2e+01) ; PlayerRight
    (Variables|TargetRotation|SetTurn (Math|Float|Clamp(Float) (- (* (Variables|TargetRotation|GetTurn) (/ (Variables|TargetRotation|GetDifference) (Variables|Default|GetTurnMultiplier))) -3e+01) -8e+01 3e+01))
    (else
      (Variables|TargetRotation|SetDifference (- (Variables|TargetRotation|GetDefaultX) (Variables|TargetRotation|GetTargetX)))
      (Variables|TargetRotation|SetTurn 1.0)
      (Variables|Default|SetTurnMultiplier 2e+01)
      (Variables|TargetRotation|SetTurn (Math|Float|Clamp(Float) (- (* (Variables|TargetRotation|GetTurn) (/ (Variables|TargetRotation|GetDifference) (Variables|Default|GetTurnMultiplier))) -3e+01) -3e+01 1.2e+02)))))

(event Custom|SetCurrentRotation
  (bind _attacklimb (Variables|Default|GetAttackLimb))
  (bind _relativerotation (Variables|/Script/Engine.SceneComponent|GetRelativeRotation _attacklimb))
  ;[0.05208 0.05208 0.05208] Attack Functions
  (Variables|TargetRotation|SetCurrentRotation (Math|Vector|MakeVector (.roll _relativerotation) 0.0 (.yaw _relativerotation))))

(event Custom|FollowPlayerTarget
  ;[0.05208 0.05208 0.05208] Attack Functions
  ;;[0.1667 0.02083 0.09256] Spike follows the player
  (bind _newtrack_0 (Timeline|TargetTimeline PlayFromStart)
    (:Update
      (CallFunction|GetDifference false)
      (if (>= _newtrack_0 1.0)
        (Transformation|SetRelativeRotation (Variables|Default|GetAttackLimb) (Math|Rotator|MakeRotator 1e+02 0.0 (Variables|TargetRotation|GetTurn)) false false)
        (else
          (Transformation|SetRelativeRotation (Variables|Default|GetAttackLimb) (Math|Rotator|MakeRotator (.x (Math|Vector|Lerp(Vector) (Variables|TargetRotation|GetCurrentRotation) (Math|Vector|MakeVector 1e+02 0.0 (Variables|TargetRotation|GetTurn)) _newtrack_0)) 0.0 (.z (Math|Vector|Lerp(Vector) (Variables|TargetRotation|GetCurrentRotation) (Math|Vector|MakeVector 1e+02 0.0 (Variables|TargetRotation|GetTurn)) _newtrack_0))) false false))))
    (:Finished
      (CallFunction|SetCurrentRotation))))

(event Custom|TargetToPlayer
  (bind _player (Variables|Default|GetPlayer))
  (bind _returnvalue (Transformation|GetActorLocation _player))
  ;[0.05208 0.05208 0.05208] Attack Functions
  ;;[0.34 0.23 0.19] Move target to player
  (Transformation|SetActorLocation (Variables|TargetRotation|GetTargetPoint) (Math|Vector|MakeVector (.x _returnvalue) (.y _returnvalue) (.z _returnvalue)) false false))

(event EventBeginPlay
  (Rendering|SetActorHiddenInGame true)
  (Collision|SetActorEnableCollision false)
  (bind _returnvalue (Actor|GetActorOfClass "/Game/ThirdPerson/Blueprints/BP_ThirdPersonCharacter.BP_ThirdPersonCharacter_C"))
  (Variables|Default|SetPlayer _returnvalue)
  (Variables|LocationTracking|SetSpikeDefaultLocation (Transformation|GetWorldLocation (Variables|Default|GetAttackLimb))))

(fn ConstructionScript
  (bind _returnvalue (Rendering|Material|CreateDynamicMaterialInstance "/Game/LevelAssets/Materials/WavyBloodMat.WavyBloodMat" "None" "None" :!class /Script/Engine.KismetMaterialLibrary))
  (bind _output_get (Variables|Default|SetWaveInst _returnvalue))
  (Rendering|Material|SetMaterial (Variables|Default|GetCentralSphere) 0 _output_get)
  (Rendering|Material|SetScalarParameterValueonMaterials (Variables|Default|GetCentralSphere) "WaveHeight" 1e+01))