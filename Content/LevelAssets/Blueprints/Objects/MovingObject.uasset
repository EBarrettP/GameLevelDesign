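; MovingObject is a level object that moves and rotates to a target transform when MoveObject is triggered, optionally starting hidden.
; MoveObject reveals the mesh, switches on the query-only box collision and captures the starting transform.
; A timeline with adjustable play rate then lerps location and rotation to the targets without sweeping, optionally spawning a smoke effect at the mesh when finished.
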(event Custom|MoveObject
  (bind _mesh (Variables|Default|GetMesh))
  (bind _returnvalue (Transformation|GetWorldTransform _mesh))
  (Components|Timeline|SetPlayRate (Variables|Default|GetMoveTimeL) (Variables|Default|GetTimelinePlayRate))
  (Variables|Default|SetStartPosition (Transformation|GetActorLocation))
  (Variables|Default|SetStartRotation (Transformation|GetActorRotation))
  (Development|SetHiddeninGame (Variables|Default|GetMesh) false false)
  (Collision|SetCollisionEnabled (Variables|Default|GetBox) "QueryOnly")
  (bind _track (Timeline|MoveTimeL PlayFromStart)
    (:Update
      (Transformation|SetActorRotation (Math|Rotator|Lerp(Rotator) (Variables|Default|GetStartRotation) (Variables|Default|GetRotationPosition) _track))
      (Transformation|SetActorLocation (Math|Vector|Lerp(Vector) (Variables|Default|GetStartPosition) (Variables|Default|GetPositionToMoveTo) _track) false false))
    (:Finished
      (if (Variables|Default|GetSpawnSmoke)
        (Niagara|SpawnSystematLocation "/Game/LevelAssets/ParticleEffects/Smoke.Smoke" (.location _returnvalue) (.rotation _returnvalue) (.scale _returnvalue))))))

(event EventBeginPlay
  (Collision|SetCollisionEnabled (Variables|Default|GetBox) "NoCollision")
  (if (Variables|Default|GetStartHidden?)
    (Development|SetHiddeninGame (Variables|Default|GetMesh) true false)))

(fn ConstructionScript)