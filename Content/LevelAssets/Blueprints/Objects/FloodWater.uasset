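; Flood water level object that rises vertically when RaiseWaterLevel is called.
; A timeline lerps the actor's Z from its height at call time to RiseHeight, keeping X and Y fixed.
; The first time the rise finishes, it moves the WavingArm1 component to a random horizontal offset at a fixed relative height and activates it, guarded by the Active flag.
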(event Custom|RaiseWaterLevel
  (bind _returnvalue (Math|Random|RandomFloatinRange -3e+01 3e+01))
  (bind _wavingarm1 (Variables|Default|GetWavingArm1))
  (bind _output_get (Variables|Default|SetStartLocation (Transformation|GetActorLocation)))
  (Variables|Default|SetStartHeight (.z _output_get))
  (bind _newtrack_0 (Timeline|RaiseTimeL PlayFromStart)
    (:Update
      (Transformation|SetActorLocation (Math|Vector|MakeVector (.x (Variables|Default|GetStartLocation)) (.y (Variables|Default|GetStartLocation)) (Math|Float|Lerp (Variables|Default|GetStartHeight) (Variables|Default|GetRise%20Height) _newtrack_0)) false false))
    (:Finished
      (if (not (Variables|Default|GetActive))
        (Transformation|SetRelativeLocation _wavingarm1 (Math|Vector|MakeVector _returnvalue _returnvalue 7e+01) false false)
        (Components|Activation|Activate _wavingarm1 false)
        (Variables|Default|SetActive true)))))

(fn ConstructionScript)