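; RodLight is a rod light actor pairing a RectLight with an emissive LightStrip mesh, switchable on or off.
; The construction script gives the strip a dynamic material tinted to the light's colour.
; Events toggle light visibility with strip glow and colour, or set a Pulse material parameter; StartOff turns it off at BeginPlay.
; SetLightColour changes only the RectLight, so the strip picks up new colours on TurnLightOn.
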(event Custom|SetLightColour
  (params (New%20Colour :type Linear%20Color%20Structure))
  (Rendering|Components|Light|SetLightColor (Variables|Default|GetRectLight) New%20Colour true))

(event Custom|TurnLightOn
  (Development|SetHiddeninGame (Variables|Default|GetRectLight) false false)
  (Rendering|Material|SetScalarParameterValueonMaterials (Variables|Default|GetLightStrip) "EmissiveStrength" 0.1)
  (Rendering|Material|SetVectorParameterValueonMaterials (Variables|Default|GetLightStrip) "Colour" (Math|Conversions|ToVector(LinearColor) (Rendering|Components|Light|GetLightColor (Variables|Default|GetRectLight)))))

(event Custom|TurnLightOff
  (Development|SetHiddeninGame (Variables|Default|GetRectLight) true false)
  (Rendering|Material|SetScalarParameterValueonMaterials (Variables|Default|GetLightStrip) "EmissiveStrength" 0.0)
  (Rendering|Material|SetVectorParameterValueonMaterials (Variables|Default|GetLightStrip) "Colour" "0.150000,0.150000,0.150000"))

(event Custom|Set%20Light%20Pulse
  (params (PulseOn :type Boolean))
  (if PulseOn
    (Rendering|Material|SetScalarParameterValueonMaterials (Variables|Default|GetLightStrip) "Pulse" 1.0)
    (else
      (Rendering|Material|SetScalarParameterValueonMaterials (Variables|Default|GetLightStrip) "Pulse" 0.0))))

(event EventBeginPlay
  (if (Variables|Default|GetStartOff)
    (CallFunction|TurnLightOff)))

(fn ConstructionScript
  (bind _returnvalue (Rendering|Material|CreateDynamicMaterialInstance (Variables|Default|GetLightStrip) 0 "/Game/LevelAssets/Materials/BasicMaterial.BasicMaterial" "None" :!class /Script/Engine.PrimitiveComponent))
  (bind _output_get (Variables|Default|SetLightStripMat _returnvalue))
  (Rendering|Material|SetMaterial (Variables|Default|GetLightStrip) 0 _output_get)
  (Rendering|Material|SetScalarParameterValueonMaterials (Variables|Default|GetLightStrip) "EmissiveStrength" 0.1)
  (Rendering|Material|SetVectorParameterValueonMaterials (Variables|Default|GetLightStrip) "Colour" (Math|Conversions|ToVector(LinearColor) (Rendering|Components|Light|GetLightColor (Variables|Default|GetRectLight)))))